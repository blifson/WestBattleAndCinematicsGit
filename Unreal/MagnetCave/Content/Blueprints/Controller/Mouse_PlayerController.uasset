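; Player controller that tracks the direction from the player character to the mouse cursor in the world.
; On BeginPlay it casts and caches the player pawn as CH_Player.
; Each Tick it traces under the cursor on the Visibility channel and normalizes the Y and Z offset from the character into MouseRotationVector, leaving out X so the direction lies in the YZ plane.
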(event `self.ReceiveBeginPlay`
  (bind _asch_player (cast `/Game/Blueprints/Characters/CH_Player` (`GameplayStatics.GetPlayerCharacter` 0)))
  (set `self.PlayerCharacter` _asch_player))

(event `self.ReceiveTick`
  (params (DeltaSeconds :type "Float (single-precision)"))
  (bind (_returnvalue_x _returnvalue_y _returnvalue_z) (`KismetMathLibrary.BreakVector` (- (`.Location` (`GameplayStatics.BreakHitResult` (`self.GetHitResultUnderCursorByChannel` "TraceTypeQuery1"))) (`self.K2_GetActorLocation` (`self.PlayerCharacter`)))))
  (set `self.MouseRotationVector` (`KismetMathLibrary.Normal` (`KismetMathLibrary.MakeVector` 0.0 _returnvalue_y _returnvalue_z))))

(fn `UserConstructionScript`)