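; BP_RocketRobot is an enemy robot that periodically fires a BP_Bomb projectile and can be destroyed by a bomb hit.
; BeginPlay starts a looping timer that calls ShootRocket, which spawns the bomb at the Arrow component's location with a set speed and prints a debug message.
; A BombHit event, with no caller in this graph, destroys the robot.
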(event `self.ReceiveBeginPlay`
  (`parent.ReceiveBeginPlay`)
  (`KismetSystemLibrary.K2_SetTimerDelegate` (delegate `ShootRocket`) 2.5 true))

(event `ShootRocket`
  (`|SpawnActorFromClass` "/Game/Blueprints/Projectile/BP_Bomb.BP_Bomb_C" (`KismetMathLibrary.MakeTransform` (`SceneComponent.K2_GetComponentLocation` (`self.Arrow`))) "Undefined" "OverrideRootScale" null true (0.0 1.0 0.0) 1000.0 null)
  (`KismetSystemLibrary.PrintString` "Shoot"))

(event `self.BombHit`
  (`self.K2_DestroyActor`))

(fn `UserConstructionScript`
  (`parent.UserConstructionScript`))