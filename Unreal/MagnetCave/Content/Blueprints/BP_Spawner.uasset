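; Spawner actor that places one instance of a configured class at its own location and respawns it after it is destroyed.
; SpawnedWasDestroyed clears the spawned flag and starts a respawn timer that calls RequestSpawn.
; RequestSpawn waits while a CH_Player overlaps the spawner, and the end of that overlap retries the deferred spawn.
; BeginPlay is unused, so nothing here triggers an initial spawn.
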(event `self.ReceiveActorBeginOverlap`
  (params (OtherActor :type "Actor Object Reference"))
  (cast `/Game/Blueprints/Characters/CH_Player` OtherActor)
  (set `self.PlayerOverlapped` true))

(event `self.ReceiveActorEndOverlap`
  (params (OtherActor :type "Actor Object Reference"))
  (cast `/Game/Blueprints/Characters/CH_Player` OtherActor)
  (set `self.PlayerOverlapped` false)
  (if (`self.WaitingForPlayerToLeave`)
    (`self.RequestSpawn`)))

(event `SpawnedWasDestroyed`
  (set `self.BeenSpawned` false)
  (`KismetSystemLibrary.K2_SetTimer` null "RequestSpawn" (`self.RespawnTime`)))

(fn `RequestSpawn`
  (if (`self.PlayerOverlapped`)
    (set `self.WaitingForPlayerToLeave` true)
    (elif (not (`self.BeenSpawned`))
      (`|SpawnActorFromClass` (`GameplayStatics.GetObjectClass` (`self.ToSpawn`)) (`KismetMathLibrary.MakeTransform` (`self.K2_GetActorLocation`)) "Undefined" "OverrideRootScale" null null)
      (set `self.BeenSpawned` true))))

(fn `UserConstructionScript`)