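; BP_Hit_MoveGrapple, stored in an OLD/CanGrapple folder, appears to be a moving grapple target driven by ProjectileMovement.
; The construction script sets velocity to the unit direction from the local origin toward the MoveTowards component's relative location.
; A Reverse event negates velocity for back-and-forth motion, but its looping timer and the Speed setup are disconnected.
; BeginPlay only calls the parent.
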(event `self.ReceiveBeginPlay`
  (`parent.ReceiveBeginPlay`))

(event `Reverse`
  (bind _projectilemovement (`self.ProjectileMovement`))
  (set `MovementComponent.Velocity` (* (`MovementComponent.Velocity` _projectilemovement) -1.0) _projectilemovement))

(fn `UserConstructionScript`
  (`parent.UserConstructionScript`)
  (bind _output_get (set `self.Direction` (`KismetMathLibrary.Conv_RotatorToVector` (`KismetMathLibrary.FindLookAtRotation` (`KismetMathLibrary.MakeVector` 0.0) (`SceneComponent.RelativeLocation` (`self.MoveTowards`))))))
  (set `MovementComponent.Velocity` _output_get (`self.ProjectileMovement`)))