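; BP_HitBase is a base Blueprint for hitable level objects, built around a Cube mesh component.
; Its construction script can turn the Cube into a wedge, scaled from height and the tangent of the angle, and can mirror it by negating yaw.
; On BeginPlay, it optionally snaps its root to the player character's X position, placing it on the player's plane while keeping Y and Z.
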(event `self.ReceiveBeginPlay`
  (bind _defaultsceneroot (`self.DefaultSceneRoot`))
  (bind (_returnvalue_x _returnvalue_y _returnvalue_z) (`KismetMathLibrary.BreakVector` (`SceneComponent.K2_GetComponentLocation` _defaultsceneroot)))
  (bind _returnvalue_x_2 (`KismetMathLibrary.BreakVector` (`self.K2_GetActorLocation` (`GameplayStatics.GetPlayerCharacter` 0))))
  (if (`self.ForceToPlayerPlane`)
    (`SceneComponent.K2_SetWorldLocation` _defaultsceneroot (`KismetMathLibrary.MakeVector` _returnvalue_x_2 _returnvalue_y _returnvalue_z) false false)))

(fn `UserConstructionScript`
  (bind _cube (`self.Cube`))
  (bind _wedgehieght (`self.WedgeHieght`))
  (bind _cube_2 (`self.Cube`))
  (`|ExecutionSequence`
    (:`then_0`
      (if (`self.Wedge`)
        (`StaticMeshComponent.SetStaticMesh` _cube "/Game/Meshes/StarterContent/Shapes/Shape_Wedge_B.Shape_Wedge_B")
        (`SceneComponent.K2_SetRelativeTransform` _cube (`KismetMathLibrary.MakeTransform` (0.0 0.0 0.0) (struct :`Yaw` -90.0) (`KismetMathLibrary.MakeVector` 1.0 _wedgehieght (* _wedgehieght (`KismetMathLibrary.DegTan` (`self.WedgeAngle`))))) false false)))
    (:`then_1`
      (if (`self.Flip`)
        (`SceneComponent.K2_SetRelativeRotation` _cube_2 (`KismetMathLibrary.MakeRotator` (.roll (`SceneComponent.RelativeRotation` _cube_2)) (.pitch (`SceneComponent.RelativeRotation` _cube_2)) (* (.yaw (`SceneComponent.RelativeRotation` _cube_2)) -1.0)) false false)))))