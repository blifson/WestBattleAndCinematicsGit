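; BP_Block is a hitable level block that can act as a lethal hazard for the player.
; On BeginPlay it optionally snaps its root to the player's X position, aligning it with the player's movement plane.
; Its Hit event kills a CH_Player when the Death flag is set.
; An unconnected collision node for ledge climbing remains, so CanClimbLedge has no effect in this graph.
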(event `self.ReceiveBeginPlay`
  (bind _defaultsceneroot (`self.DefaultSceneRoot`))
  (bind (_returnvalue_x _returnvalue_y _returnvalue_z) (`KismetMathLibrary.BreakVector` (`SceneComponent.K2_GetComponentLocation` _defaultsceneroot)))
  (bind _returnvalue_x_2 (`KismetMathLibrary.BreakVector` (`self.K2_GetActorLocation` (`GameplayStatics.GetPlayerCharacter` 0))))
  (if (`self.ForceToPlayerPlane`)
    (`SceneComponent.K2_SetWorldLocation` _defaultsceneroot (`KismetMathLibrary.MakeVector` _returnvalue_x_2 _returnvalue_y _returnvalue_z) false false)))

(event `self.ReceiveHit`
  (params (MyComp :type "PrimitiveComponent Object Reference") (Other :type "Actor Object Reference") (OtherComp :type "PrimitiveComponent Object Reference") (bSelfMoved :type Boolean) (HitLocation :type "Vector Structure") (HitNormal :type "Vector Structure") (NormalImpulse :type "Vector Structure") (Hit :type "HitResult Structure (by ref)"))
  (bind _asch_player (cast `/Game/Blueprints/Characters/CH_Player` Other))
  (if (`self.Death`)
    (`/Game/Blueprints/Characters/CH_Player.Death` _asch_player 0 (0.0 0.0 0.0))))

(fn `UserConstructionScript`)