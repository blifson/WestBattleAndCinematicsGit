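; BP_Hit_MoveGrapple is a moving hittable object, apparently a grapple target, that travels back and forth along a straight path.
; The construction script configures its ProjectileMovement component from the Speed and Direction variables, capping max speed at the initial speed.
; On BeginPlay a looping timer negates the velocity at each ReverseEvery interval, producing the ping-pong motion without using Tick.
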(event `self.ReceiveBeginPlay`
  (`parent.ReceiveBeginPlay`)
  (`KismetSystemLibrary.K2_SetTimerDelegate` (delegate `Reverse`) (`self.ReverseEvery`) true))

(event `Reverse`
  (bind _projectilemovement (`self.ProjectileMovement`))
  (set `MovementComponent.Velocity` (* (`MovementComponent.Velocity` _projectilemovement) -1.0) _projectilemovement))

(fn `UserConstructionScript`
  (bind _projectilemovement (`self.ProjectileMovement`))
  (`parent.UserConstructionScript`)
  (bind _output_get (set `ProjectileMovementComponent.InitialSpeed` (`self.Speed`) _projectilemovement))
  (set `ProjectileMovementComponent.MaxSpeed` _output_get _projectilemovement)
  (set `MovementComponent.Velocity` (`self.Direction`) _projectilemovement))