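; BP_CollectableBase is a collectable actor, named as a base class, that lines itself up with the player's plane.
; On BeginPlay it copies the X coordinate of player pawn 0 and keeps its own Y and Z.
; A disconnected chain, which never runs, would refill a CH_Player's Grip to GripMax when below it and then destroy the collectable.
; Tick and the construction script do nothing.
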(event `self.ReceiveBeginPlay`
  (bind (_returnvalue_x _returnvalue_y _returnvalue_z) (`KismetMathLibrary.BreakVector` (`self.K2_GetActorLocation`)))
  (bind _returnvalue_x_2 (`KismetMathLibrary.BreakVector` (`self.K2_GetActorLocation` (`GameplayStatics.GetPlayerPawn` 0))))
  (`self.K2_SetActorLocation` (`KismetMathLibrary.MakeVector` _returnvalue_x_2 _returnvalue_y _returnvalue_z)))

(fn `UserConstructionScript`)