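; Base interactable Blueprint, spawned by a parent spawner and collected when the player touches it.
; On BeginPlay it snaps its X to the player pawn's X, keeping its own Y and Z.
; Overlap with CH_Player registers the spawner as collected on the player, and destruction notifies that spawner.
; An unconnected leftover branch would refill the player's Grip and destroy the actor.
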(event `self.ReceiveBeginPlay`
  (bind (_returnvalue_x _returnvalue_y _returnvalue_z) (`KismetMathLibrary.BreakVector` (`self.K2_GetActorLocation`)))
  (bind _returnvalue_x_2 (`KismetMathLibrary.BreakVector` (`self.K2_GetActorLocation` (`GameplayStatics.GetPlayerPawn` 0))))
  (`self.K2_SetActorLocation` (`KismetMathLibrary.MakeVector` _returnvalue_x_2 _returnvalue_y _returnvalue_z)))

(event `self.ReceiveDestroyed`
  (bind _parentspawner (`self.ParentSpawner`))
  (`/Engine/EditorBlueprintResources/StandardMacros.IsValid` _parentspawner
    (:`Is Valid`
      (`/Game/Blueprints/Interactables/SpawnablePickups/BP_PickupSpawner.SpawnedWasDestroyed` _parentspawner))))

(event `self.ReceiveActorBeginOverlap`
  (params (OtherActor :type "Actor Object Reference"))
  (bind _parentspawner (`self.ParentSpawner`))
  (`/Engine/EditorBlueprintResources/StandardMacros.IsValid` _parentspawner
    (:`Is Valid`
      (bind _asch_player (cast `/Game/Blueprints/Characters/CH_Player` OtherActor))
      (`/Game/Blueprints/Characters/CH_Player.AddCollectedSpawner` _asch_player _parentspawner))))

(fn `UserConstructionScript`)