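; BP_GripRefill is a pickup that refills the player's grip and shots when touched.
; On actor overlap it casts the other actor to CH_Player, sets Grip and ShotsCur to their maximum values, then destroys itself.
; BeginPlay and Tick are disabled, and the construction script only calls its parent.
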(event `self.ReceiveActorBeginOverlap`
  (params (OtherActor :type "Actor Object Reference"))
  (`parent.ReceiveActorBeginOverlap` OtherActor)
  (bind _asch_player (cast `/Game/Blueprints/Characters/CH_Player` OtherActor))
  (if true
    (set `/Game/Blueprints/Characters/CH_Player.Grip` (`/Game/Blueprints/Characters/CH_Player.GripMax` _asch_player) _asch_player)
    (set `/Game/Blueprints/Characters/CH_Player.ShotsCur` (`/Game/Blueprints/Characters/CH_Player.ShotsMax` _asch_player) _asch_player)
    (`self.K2_DestroyActor`)))

(fn `UserConstructionScript`
  (`parent.UserConstructionScript`))