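; BP_SecretCoin is a collectible secret coin that the player picks up by overlapping it.
; While active, an overlap by CH_Player increments that player's CoinsHeld and adds the coin to its CoinsBeforeCheckpoint list.
; SetActiveCoin then clears the Active flag and hides the mesh and its children instead of destroying the actor, so the same function can re-enable the coin.
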(event `self.ReceiveActorBeginOverlap`
  (params (OtherActor :type "Actor Object Reference"))
  (if (`self.Active`)
    (bind _asch_player (cast `/Game/Blueprints/Characters/CH_Player` OtherActor))
    (`/Engine/EditorBlueprintResources/StandardMacros.IncrementInt` (`/Game/Blueprints/Characters/CH_Player.CoinsHeld` _asch_player)
      (:`  `
        (`KismetArrayLibrary.Array_Add` (`/Game/Blueprints/Characters/CH_Player.CoinsBeforeCheckpoint` _asch_player) self)
        (`self.SetActiveCoin` false)))))

(fn `SetActiveCoin`
  (params (Active :type Boolean :default true))
  (bind _output_get (set `self.Active` Active))
  (`SceneComponent.SetVisibility` (`self.StaticMesh`) _output_get true))

(fn `UserConstructionScript`)