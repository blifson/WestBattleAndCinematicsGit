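; Enemy projectile that kills the player on contact and can be bounced back by a magnet projectile.
; Construction script sets its movement from Direction and Speed.
; On sphere overlap, an eligible magnet hit reverses velocity once, boosts speed limits, resets lifespan and consumes the magnet projectile.
; Other non-magnet overlaps destroy it; older Hit-based logic is left disconnected.
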(event `self.ReceiveHit`
  (params (MyComp :type "PrimitiveComponent Object Reference") (Other :type "Actor Object Reference") (OtherComp :type "PrimitiveComponent Object Reference") (bSelfMoved :type Boolean) (HitLocation :type "Vector Structure") (HitNormal :type "Vector Structure") (NormalImpulse :type "Vector Structure") (Hit :type "HitResult Structure (by ref)")))

(event `self.ReceiveDestroyed`
  (`KismetSystemLibrary.PrintString` "Boom"))

(event `self.SphereCollision.OnComponentBeginOverlap`
  (params (OverlappedComponent :type "PrimitiveComponent Object Reference") (OtherActor :type "Actor Object Reference") (OtherComp :type "PrimitiveComponent Object Reference") (OtherBodyIndex :type Integer) (bFromSweep :type Boolean) (SweepResult :type "HitResult Structure (by ref)"))
  (bind _projectilemovement (`self.ProjectileMovement`))
  (bind _mesh (`self.Mesh`))
  (bind (_relativerotation_roll _relativerotation_pitch _relativerotation_yaw) (`KismetMathLibrary.BreakRotator` (`SceneComponent.RelativeRotation` _mesh)))
  (bind _asch_player (cast `/Game/Blueprints/Characters/CH_Player` OtherActor)
    (:`then`
      (`/Game/Blueprints/Characters/CH_Player.Death` _asch_player 0 (0.0 0.0 0.0))
      (`self.K2_DestroyActor` :!label _label))
    (:`CastFailed`
      (bind _asbp_magnet_projectile (cast `/Game/Blueprints/Projectile/BP_MagnetProjectile` OtherActor)
        (:`then`
          (if (not (`self.IgnoreMagnetHit`))
            (if (and (not (`self.Reversed`)) (`self.MagnetReverses`))
              (`self.SetLifeSpan` (`self.Lifespan`))
              (`SceneComponent.K2_SetRelativeRotation` _mesh (`KismetMathLibrary.MakeRotator` _relativerotation_roll _relativerotation_pitch (* _relativerotation_yaw -1.0)) false false)
              (`self.K2_SetActorRotation` (`KismetMathLibrary.MakeRotator` 0.0))
              (set `MovementComponent.Velocity` (* (`MovementComponent.Velocity` _projectilemovement) -1.0) _projectilemovement)
              (set `self.Reversed` true)
              (set `ProjectileMovementComponent.InitialSpeed` (* (`ProjectileMovementComponent.InitialSpeed` _projectilemovement) 1.5) _projectilemovement)
              (set `ProjectileMovementComponent.MaxSpeed` (* (`ProjectileMovementComponent.MaxSpeed` _projectilemovement) 1.5) _projectilemovement)
              (`/Engine/EditorBlueprintResources/StandardMacros.IsValid` _asbp_magnet_projectile
                (:`Is Valid`
                  (`self.K2_DestroyActor` _asbp_magnet_projectile))))))
        (:`CastFailed`
          (goto _label))))))

(fn `UserConstructionScript`
  (bind _projectilemovement (`self.ProjectileMovement`))
  (set `MovementComponent.Velocity` (`self.Direction`) _projectilemovement)
  (bind _output_get (set `ProjectileMovementComponent.MaxSpeed` (`self.Speed`) _projectilemovement))
  (set `ProjectileMovementComponent.InitialSpeed` _output_get _projectilemovement))