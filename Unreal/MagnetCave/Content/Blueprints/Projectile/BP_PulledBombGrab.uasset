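; BP_PulledBombGrab is a projectile that homes in on the player and adds one bomb to them when it is destroyed.
; On BeginPlay it caches player 0 as CH_Player and sets that character's root component as the homing target of its ProjectileMovement.
; Overlapping a CH_Player destroys it.
; The bomb is granted in the Destroyed event, so destruction by other causes also triggers AddBomb.
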(event `self.ReceiveBeginPlay`
  (bind _projectilemovement (`self.ProjectileMovement`))
  (bind _asch_player (cast `/Game/Blueprints/Characters/CH_Player` (`GameplayStatics.GetPlayerCharacter` 0)))
  (set `self.Player` _asch_player)
  (set `ProjectileMovementComponent.bIsHomingProjectile` true _projectilemovement)
  (set `ProjectileMovementComponent.HomingTargetComponent` (`Actor.RootComponent` (`self.Player`)) _projectilemovement))

(event `self.ReceiveActorBeginOverlap`
  (params (OtherActor :type "Actor Object Reference"))
  (cast `/Game/Blueprints/Characters/CH_Player` OtherActor)
  (`self.K2_DestroyActor`))

(event `self.ReceiveDestroyed`
  (`/Game/Blueprints/Characters/CH_Player.AddBomb` (`self.Player`) 1))

(event `self.ReceiveTick`
  (params (DeltaSeconds :type "Float (single-precision)")))

(fn `UserConstructionScript`)