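; BP_Bomb is a bomb projectile fired by either side, with Direction and Speed set on its movement at construction.
; Its damage sphere breaks destructible blocks, then HurtHero picks a macro: enemy mode kills the player, player mode calls BombHit on enemies.
; ToBeDestroyed lets it pass its own side; otherwise most hits explode it.
; A separate pickup sphere lets magnet projectiles turn it into player ammo with a different effect.
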(event `self.DamageSphereCollision.OnComponentBeginOverlap`
  (params (OverlappedComponent :type "PrimitiveComponent Object Reference") (OtherActor :type "Actor Object Reference") (OtherComp :type "PrimitiveComponent Object Reference") (OtherBodyIndex :type Integer) (bFromSweep :type Boolean) (SweepResult :type "HitResult Structure (by ref)"))
  (bind _returnvalue (select `int` (`self.ParticleIndex`) :`0` "/Game/Particles/FXVarietyPack/Particles/P_ky_explosion.P_ky_explosion" :`1` "/Game/Particles/FXVarietyPack/Particles/P_ky_waterBallHit.P_ky_waterBallHit" :!type "ParticleSystem Object Reference"))
  (`/Engine/EditorBlueprintResources/StandardMacros.IsValid` OtherActor
    (:`Is Valid`
      (if (!= OtherActor self)
        (set `self.ToBeDestroyed` true)
        ;[1 1 1] Cases where it doesn't matter which state the bomb is in.
        (bind _asbp_block (cast `/Game/Blueprints/Hitable/BP_Block` OtherActor)
          (:`then`
            (if (`/Game/Blueprints/Hitable/BP_Block.Destructable` _asbp_block)
              (`self.K2_DestroyActor` _asbp_block)))
          (:`CastFailed`
            (cast `/Game/Blueprints/Projectile/BP_MagnetProjectile` OtherActor ; Make this get ignored, since it's handled by PickupSphereCollision
              (:`CastFailed`
                (if (`self.HurtHero`)
                  (`self.EnemyControlledMode` OtherActor
                    (:`Output`
                      _))
                  (else
                    (`self.PlayerControlledMode` OtherActor
                      (:`Output`
                        _))))))))
        (if (`self.ToBeDestroyed`)
          (`/Engine/EditorBlueprintResources/StandardMacros.IsValid` _returnvalue :!label _label
            (:`Is Valid`
              (`GameplayStatics.SpawnEmitterAtLocation` _returnvalue (`self.K2_GetActorLocation`)))
            (:`Is Not Valid`
              _))
          (`self.K2_DestroyActor`))))))

(event `self.PickupSphereCollision.OnComponentBeginOverlap`
  (params (OverlappedComponent :type "PrimitiveComponent Object Reference") (OtherActor :type "Actor Object Reference") (OtherComp :type "PrimitiveComponent Object Reference") (OtherBodyIndex :type Integer) (bFromSweep :type Boolean) (SweepResult :type "HitResult Structure (by ref)"))
  (`/Engine/EditorBlueprintResources/StandardMacros.IsValid` OtherActor
    (:`Is Valid`
      (if (!= null self)
        (bind _asbp_magnet_projectile (cast `/Game/Blueprints/Projectile/BP_MagnetProjectile` OtherActor))
        (`self.K2_DestroyActor` _asbp_magnet_projectile)
        (bind _asch_player (cast `/Game/Blueprints/Characters/CH_Player` (`GameplayStatics.GetPlayerCharacter` 0)))
        (`/Game/Blueprints/Characters/CH_Player.BombAdd` _asch_player)
        (set `self.ParticleIndex` 1)
        (goto _label)))))

(fn `UserConstructionScript`
  (bind _projectilemovement (`self.ProjectileMovement`))
  (set `MovementComponent.Velocity` (`self.Direction`) _projectilemovement)
  (bind _output_get (set `ProjectileMovementComponent.InitialSpeed` (`self.Speed`) _projectilemovement))
  (set `ProjectileMovementComponent.MaxSpeed` _output_get _projectilemovement))