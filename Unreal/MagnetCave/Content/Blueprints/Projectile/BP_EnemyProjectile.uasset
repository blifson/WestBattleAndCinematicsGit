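; BP_EnemyProjectile is an enemy projectile that kills the player on contact.
; The construction script feeds its Direction and Speed variables into ProjectileMovement as velocity, initial speed and max speed.
; On Hit, it calls Death on a CH_Player with its own location and destroys itself, also destroys itself on a BP_Block, and ignores other actors.
; Debug prints show the hit actor's name and "Boom" on destruction.
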(event `self.ReceiveHit`
  (params (MyComp :type "PrimitiveComponent Object Reference") (Other :type "Actor Object Reference") (OtherComp :type "PrimitiveComponent Object Reference") (bSelfMoved :type Boolean) (HitLocation :type "Vector Structure") (HitNormal :type "Vector Structure") (NormalImpulse :type "Vector Structure") (Hit :type "HitResult Structure (by ref)"))
  (`KismetSystemLibrary.PrintString` (`KismetSystemLibrary.GetDisplayName` Other))
  (bind _asch_player (cast `/Game/Blueprints/Characters/CH_Player` Other)
    (:`then`
      (`/Game/Blueprints/Characters/CH_Player.Death` _asch_player 0 (`self.K2_GetActorLocation`)))
    (:`CastFailed`
      (cast `/Game/Blueprints/Hitable/BP_Block` Other)))
  (`self.K2_DestroyActor`))

(event `self.ReceiveDestroyed`
  (`KismetSystemLibrary.PrintString` "Boom"))

(fn `UserConstructionScript`
  (bind _projectilemovement (`self.ProjectileMovement`))
  (set `MovementComponent.Velocity` (`self.Direction`) _projectilemovement)
  (bind _output_get (set `ProjectileMovementComponent.MaxSpeed` (`self.Speed`) _projectilemovement))
  (set `ProjectileMovementComponent.InitialSpeed` _output_get _projectilemovement))