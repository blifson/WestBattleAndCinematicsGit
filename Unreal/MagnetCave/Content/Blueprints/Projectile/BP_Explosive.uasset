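; Explosive projectile that breaks destructible objects on impact.
; The construction script sets the projectile movement velocity from its Direction variable.
; Hits on CH_Player or BP_InterBase actors are ignored; any other hit destroys the projectile, first destroying the target if it is a BP_HitBase flagged Destructable.
; Whenever the projectile is destroyed, it spawns an explosion particle effect at its location.
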(event `self.ReceiveHit`
  (params (MyComp :type "PrimitiveComponent Object Reference") (Other :type "Actor Object Reference") (OtherComp :type "PrimitiveComponent Object Reference") (bSelfMoved :type Boolean) (HitLocation :type "Vector Structure") (HitNormal :type "Vector Structure") (NormalImpulse :type "Vector Structure") (Hit :type "HitResult Structure (by ref)"))
  (cast `/Game/Blueprints/Characters/CH_Player` Other
    (:`CastFailed`
      (cast `/Game/Blueprints/Interactables/BP_InterBase` Other
        (:`CastFailed`
          (bind _asbp_hit_base (cast `/Game/Blueprints/Hitable/BP_HitBase` Other)
            (:`then`
              (if (`/Game/Blueprints/Hitable/BP_HitBase.Destructable` _asbp_hit_base)
                (`self.K2_DestroyActor` _asbp_hit_base)))
            (:`CastFailed`
              _))
          (`self.K2_DestroyActor`))))))

(event `self.ReceiveDestroyed`
  (`GameplayStatics.SpawnEmitterAtLocation` "/Game/Meshes/StarterContent/Particles/P_Explosion.P_Explosion" (`self.K2_GetActorLocation`)))

(fn `UserConstructionScript`
  (set `MovementComponent.Velocity` (`self.Direction`) (`self.ProjectileMovement`)))