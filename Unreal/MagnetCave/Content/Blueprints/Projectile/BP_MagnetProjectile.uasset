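; Magnet projectile that travels along a set Direction and acts as the player's grapple shot.
; On hit it ignores the player and BP_InterBase, calls MagnetHit on enemies, triggers the player's grapple on grabbable targets beyond a minimum travel distance, or spawns impact particles on other surfaces.
; It destroys itself after those hits or when Tick finds it off-screen beyond a margin, and clears the player's active-projectile flag when destroyed.
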(event `self.ReceiveBeginPlay`
  (set `self.StartingPosition` (`self.K2_GetActorLocation`))
  (bind _asch_player (cast `/Game/Blueprints/Characters/CH_Player` (`GameplayStatics.GetPlayerCharacter` 0)))
  (set `self.Player` _asch_player))

(event `self.ReceiveDestroyed`
  (`/Game/Blueprints/Characters/CH_Player.SetActiveMagnetProjectile` (`self.Player`) false))

(event `self.ReceiveHit`
  (params (MyComp :type "PrimitiveComponent Object Reference") (Other :type "Actor Object Reference") (OtherComp :type "PrimitiveComponent Object Reference") (bSelfMoved :type Boolean) (HitLocation :type "Vector Structure") (HitNormal :type "Vector Structure") (NormalImpulse :type "Vector Structure") (Hit :type "HitResult Structure (by ref)"))
  (cast `/Game/Blueprints/Characters/CH_Player` Other
    (:`CastFailed`
      (cast `/Game/Blueprints/Interactables/BP_InterBase` Other
        (:`CastFailed`
          (bind _asbp_enemy_base (cast `/Game/Blueprints/Enemy/BP_EnemyBase` Other)
            (:`then`
              (`/Game/Blueprints/Enemy/BP_EnemyBase.MagnetHit` _asbp_enemy_base))
            (:`CastFailed`
              (bind _asbp_hitb_cn_grb (cast `/Game/Blueprints/Hitable/OLD/CanGrapple/BP_HitbCnGrb` Other)
                (:`then`
                  (if (>= (`KismetMathLibrary.Vector_Distance` (`self.StartingPosition`) (`self.K2_GetActorLocation`)) (`self.MinDistance`)) :!label _label
                    (`/Game/Blueprints/Characters/CH_Player.GrappleCollisionDetected` (`self.Player`) _asbp_hitb_cn_grb HitLocation)))
                (:`CastFailed`
                  (bind _asbp_block (cast `/Game/Blueprints/Hitable/BP_Block` Other)
                    (:`then`
                      (if (`/Game/Blueprints/Hitable/BP_Block.Grabable` _asbp_block)
                        (goto _label)
                        (else
                          _)))
                    (:`CastFailed`
                      _))
                  (`GameplayStatics.SpawnEmitterAtLocation` "/Game/Particles/FXVarietyPack/Particles/P_ky_hit2.P_ky_hit2" HitLocation)))))
          (`self.K2_DestroyActor`))))))

(event `self.ReceiveTick`
  (params (DeltaSeconds :type "Float (single-precision)"))
  (bind (_returnvalue_x _returnvalue_y) (`KismetMathLibrary.BreakVector2D` (`WidgetLayoutLibrary.GetViewportSize`)))
  (bind _outcamoffset (`self.OutCamOffset`))
  (bind _returnvalue (- 0.0 (`self.OutCamOffset`)))
  (bind _screenlocation (`PlayerController.ProjectWorldLocationToScreen` (`GameplayStatics.GetPlayerController` 0) (`self.K2_GetActorLocation`) false))
  ;[1 1 1] Destroy projectile if it leaves view of camera
  (if (not (and (> (`KismetMathLibrary.BreakVector2D` _screenlocation) _returnvalue) (> (`.Y` (`KismetMathLibrary.BreakVector2D` _screenlocation)) _returnvalue) (< (`KismetMathLibrary.BreakVector2D` _screenlocation) (+ _returnvalue_x _outcamoffset)) (< (`.Y` (`KismetMathLibrary.BreakVector2D` _screenlocation)) (+ _outcamoffset _returnvalue_y))))
    (`self.K2_DestroyActor`)))

(fn `UserConstructionScript`
  (set `MovementComponent.Velocity` (`self.Direction`) (`self.ProjectileMovement`)))