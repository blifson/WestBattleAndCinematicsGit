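; Grapple line actor that draws a cable, GrappleLine, out to a fired projectile.
; FireBeam stores the projectile and activates the beam, then Tick sets the cable's end location to the projectile's world location until Attached is true.
; TurnOffBeam hides the cable and resets its length, width and end location, but leaves BeamActive unchanged.
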(event `self.ReceiveBeginPlay`)

(event `self.ReceiveTick`
  (params (DeltaSeconds :type "Float (single-precision)"))
  (if (`self.BeamActive`)
    (if (not (`self.Attached`))
      (`/Engine/EditorBlueprintResources/StandardMacros.IsValid` (`self.Projectile`)
        (:`Is Valid`
          (set `CableComponent.EndLocation` (`self.K2_GetActorLocation` (`self.Projectile`)) (`self.GrappleLine`)))))))

(fn `FireBeam`
  (params (Projectile :type "Actor Object Reference"))
  (set `self.Projectile` Projectile)
  (set `self.BeamActive` true))

(fn `TurnOffBeam`
  (bind _grappleline (`self.GrappleLine`))
  (`SceneComponent.SetVisibility` _grappleline false false)
  (set `CableComponent.CableLength` 0.0 _grappleline)
  (set `CableComponent.CableWidth` 6.0 _grappleline)
  (set `CableComponent.EndLocation` (0.0 0.0 40.0) _grappleline))

(fn `UserConstructionScript`)